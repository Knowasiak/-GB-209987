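; Nav link proxy that makes zombie agents jump to the link destination when they reach the smart link.
; SmartLinkReached casts the agent to three zombie classes, but the launch sequence runs only if the ZombieCharacterBoss cast succeeds.
; The sequence calls LaunchCharacter on each cast result, overriding velocity.
; Three identical helper functions compute the ballistic arc from JumpDuration and hard-coded gravity.
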(event `self.ReceiveSmartLinkReached`
  (params (Agent :type "Actor Object Reference") (Destination :type "Vector Structure (by ref)"))
  (bind _jumpduration (`self.JumpDuration`))
  (bind _aszombie_character (cast `/Game/Girl_Soldier/ZombieCharacter` Agent)
    (:`then`
      _)
    (:`CastFailed`
      _))
  (bind _aszombie_character_2 (cast `/Game/Girl_Soldier/ZombieCharacter2` Agent)
    (:`then`
      _)
    (:`CastFailed`
      _))
  (bind _aszombie_character_boss (cast `/Game/Girl_Soldier/ZombieBossMesh/ZombieCharacterBoss` Agent))
  (`|ExecutionSequence`
    (:`then_0`
      (bind _velocity (`self.Calculate Velocity` Destination (`self.K2_GetActorLocation` _aszombie_character) _jumpduration))
      (`Character.LaunchCharacter` _aszombie_character _velocity true true))
    (:`then_1`
      (bind _velocity_2 (`self.Calculate Velocity_1` Destination (`self.K2_GetActorLocation` _aszombie_character_2) _jumpduration))
      (`Character.LaunchCharacter` _aszombie_character_2 _velocity_2 true true))
    (:`then_2`
      (bind _velocity_3 (`self.Calculate Velocity_2` Destination (`self.K2_GetActorLocation` _aszombie_character_boss) _jumpduration))
      (`Character.LaunchCharacter` _aszombie_character_boss _velocity_3 true true))))

(fn `Calculate Velocity`
  (params (DestinationLocation :type "Vector Structure") (StartingLocation :type "Vector Structure") (Duration :type "Float (double-precision)"))
  (returns (Velocity :type "Vector Structure"))
  (bind _induration (`self.InDuration`))
  (set `self.InDuration` Duration)
  (return (`KismetMathLibrary.MakeVector` (/ (- (.x DestinationLocation) (.x StartingLocation)) _induration) (/ (- (.y DestinationLocation) (.y StartingLocation)) _induration) (/ (- (.z DestinationLocation) (+ (.z StartingLocation) (* (`KismetMathLibrary.Square` (`self.InDuration`)) -0.5 982.0))) (`self.InDuration`)))))

(fn `Calculate Velocity_1`
  (params (DestinationLocation :type "Vector Structure") (StartingLocation :type "Vector Structure") (Duration :type "Float (double-precision)"))
  (returns (Velocity :type "Vector Structure"))
  (bind _induration (`self.InDuration`))
  (set `self.InDuration` Duration)
  (return (`KismetMathLibrary.MakeVector` (/ (- (.x DestinationLocation) (.x StartingLocation)) _induration) (/ (- (.y DestinationLocation) (.y StartingLocation)) _induration) (/ (- (.z DestinationLocation) (+ (.z StartingLocation) (* (`KismetMathLibrary.Square` (`self.InDuration`)) -0.5 982.0))) (`self.InDuration`)))))

(fn `Calculate Velocity_2`
  (params (DestinationLocation :type "Vector Structure") (StartingLocation :type "Vector Structure") (Duration :type "Float (double-precision)"))
  (returns (Velocity :type "Vector Structure"))
  (bind _induration (`self.InDuration`))
  (set `self.InDuration` Duration)
  (return (`KismetMathLibrary.MakeVector` (/ (- (.x DestinationLocation) (.x StartingLocation)) _induration) (/ (- (.y DestinationLocation) (.y StartingLocation)) _induration) (/ (- (.z DestinationLocation) (+ (.z StartingLocation) (* (`KismetMathLibrary.Square` (`self.InDuration`)) -0.5 982.0))) (`self.InDuration`)))))

(fn `UserConstructionScript`)